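; Checkpoint actor assigned to one of two players, with its particle color set from PlayerRef on begin play.
; When a ThirdPersonCharacter with the matching PlayerId overlaps it, it adds a point through the DataBase actor, plays a sound and destroys itself.
; SetMultiplier applies a size multiplier for five seconds, which Tick blends at a fixed alpha into the particle cylinder radius and trigger box Y/Z scale.
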(event Custom|SetMultiplier
  (params (size :type Float%20%28single-precision%29))
  (Variables|Default|Setmultiplier size)
  (Utilities|FlowControl|Delay 5.0)
  (Variables|Default|Setmultiplier 1.0))

(event EventBeginPlay
  (bind _particlesystem (Variables|Default|GetParticleSystem))
  (switch int (Variables|Default|GetplayerRef)
    (:1
      (Effects|Components|ParticleSystem|SetColorParameter _particlesystem "NewColor" "(R=0.080761,G=0.310571,B=1.000000,A=1.000000)"))
    (:2
      (Effects|Components|ParticleSystem|SetColorParameter _particlesystem "NewColor" "(R=0.953915,G=1.000000,B=0.195016,A=1.000000)"))))

(event Collision|EventActorBeginOverlap
  (params (OtherActor :type Actor%20Object%20Reference))
  ;[1 1 1] check if overlaping player
  (Variables|Default|SetSourceActorObject OtherActor)
  (bind _asactor (Utilities|Casting|CastToActorClass (Utilities|GetClass OtherActor)))
  (if (== _asactor "/Game/Blueprints/ThirdPersonCharacter.ThirdPersonCharacter_C")
    (bind _asthird_person_character (Utilities|Casting|CastToThirdPersonCharacter (Variables|Default|GetSourceActorObject)))
    ;[1 1 1] Points Management
    (if (== (Variables|Default|GetplayerRef) (Variables|/Game/Blueprints/ThirdPersonCharacter.ThirdPersonCharacter_C|GetplayerId _asthird_person_character))
      (bind _outactors (Actor|GetAllActorsOfClass "/Game/Blueprints/DataBase.DataBase_C"))
      (Default|AddPoints (Utilities|Array|Get(acopy) _outactors) 1)
      (Actor|DestroyActor)
      (Audio|PlaySoundatLocation "/Game/Sounds/CheckPoint.CheckPoint" (Transformation|GetWorldLocation (Variables|Default|GetParentMesh))))))

(event EventTick
  (params (DeltaSeconds :type Float%20%28single-precision%29))
  (bind _particleradius (Variables|Default|GetparticleRadius))
  (bind _bboxscale (Variables|Default|GetbBoxScale))
  (bind _multiplier (Variables|Default|Getmultiplier))
  (bind _returnvalue (* _bboxscale _multiplier))
  (bind (_x _y _z) (Math|Vector|BreakVector _returnvalue))
  (Effects|Components|ParticleSystem|SetFloatParameter (Variables|Default|GetParticleSystem) "CylinderRadius" (Math|Float|Lerp _particleradius (* _particleradius (Variables|Default|Getmultiplier)) 0.1))
  (Transformation|SetRelativeScale3D (Variables|Default|GetBox) (Math|Vector|Lerp(Vector) _bboxscale (Math|Vector|MakeVector 1.0 _y _z) 0.1)))

(fn ConstructionScript)