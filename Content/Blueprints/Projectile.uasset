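; Projectile Blueprint that collects red, blue and yellow pickups on overlap, awarding points by color and destroying the pickup.
; It identifies pickups by switching on class display name, so renaming those Blueprints breaks matching.
; AddPoints sends the score to DatabaseReference and the first DataBase actor found, then prints it on screen.
; Logic that sets DatabaseReference and self-destroys after a delay on authority is disconnected and never runs.
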(event Custom|AddPoints
  (params (PointsAmount :type Integer))
  ;[1 1 1] AddPoints
  (bind _outactors (Actor|GetAllActorsOfClass "/Game/Blueprints/DataBase.DataBase_C"))
  (Default|AddPoints (Variables|Default|GetDatabaseReference) PointsAmount)
  (Development|PrintString (Utilities|String|Append "+ " (Utilities|String|ToString(Integer) PointsAmount) " pts") true true "(R=1.000000,G=0.528357,B=0.000000,A=1.000000)" 5.0))

(event EventBeginPlay)

(event EventTick
  (params (DeltaSeconds :type Float%20%28single-precision%29)))

(event Collision|EventActorBeginOverlap
  (params (OtherActor :type Actor%20Object%20Reference))
  ;[1 1 1] OverlapSourceSwitch/Case
  (Variables|Default|SetSourceActorObject OtherActor)
  (bind _asactor (Utilities|Casting|CastToActorClass (Utilities|GetClass OtherActor)))
  (switch string (Utilities|GetClassDisplayName _asactor)
    (:bp_pickUpRed_c
      (Development|PrintString "Player: Red" true true "(R=1.000000,G=0.528357,B=0.000000,A=1.000000)")
      (CallFunction|AddPoints 1)
      (Actor|DestroyActor (Variables|Default|GetSourceActorObject)))
    (:bp_pickUpBlue_c
      (Development|PrintString "Player: Blue" true true "(R=1.000000,G=0.528357,B=0.000000,A=1.000000)")
      (CallFunction|AddPoints 2)
      (Actor|DestroyActor (Variables|Default|GetSourceActorObject)))
    (:bp_pickUpYellow_c
      (Development|PrintString "Player: Yellow" true true "(R=1.000000,G=0.528357,B=0.000000,A=1.000000)")
      (CallFunction|AddPoints 3)
      (Actor|DestroyActor (Variables|Default|GetSourceActorObject)))))

(fn ConstructionScript)