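; Actor Blueprint whose static mesh starts at an initial uniform scale and grows toward a target scale once ScaleUp is called.
; ScaleUp only sets a flag; Tick then lerps the scale with an alpha that itself lerps toward a target alpha, easing per frame independently of delta time.
; Scaling stops once the size passes 90% of the target, printing a debug message.
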(event EventBeginPlay
  (bind _initialscale (Variables|Default|GetinitialScale))
  (Transformation|SetRelativeScale3D (Variables|Default|GetStaticMesh) (Math|Vector|MakeVector _initialscale _initialscale _initialscale)))

(event EventActorBeginOverlap
  (params (OtherActor :type Actor%20Object%20Reference)))

(event EventTick
  (params (DeltaSeconds :type Float%20%28single-precision%29))
  (if (Variables|Default|GetallowScaling)
    (Variables|Default|SetinitialScale (Math|Float|Lerp (Variables|Default|GetinitialScale) (Variables|Default|GettargetScale) (Variables|Default|GetinitialAlpha)))
    (Variables|Default|SetinitialAlpha (Math|Float|Lerp (Variables|Default|GetinitialAlpha) (Variables|Default|GettargetAlpha) 0.01))
    (Transformation|SetRelativeScale3D (Variables|Default|GetStaticMesh) (Math|Vector|MakeVector (Variables|Default|GetinitialScale) (Variables|Default|GetinitialScale) (Variables|Default|GetinitialScale)))
    (if (> (Variables|Default|GetinitialScale) (* (Variables|Default|GettargetScale) 0.9))
      (Variables|Default|SetallowScaling false)
      (Development|PrintString "StopScaling" true true "(R=1.000000,G=0.000000,B=0.053325,A=1.000000)"))))

(fn ConstructionScript)

(fn ScaleUp
  (Variables|Default|SetallowScaling true)
  (return))