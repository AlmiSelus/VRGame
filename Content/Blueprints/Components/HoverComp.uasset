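; Hover component that makes its owning actor float above surfaces using physics forces.
; BeginPlay enables physics simulation on the owner's first primitive component.
; Each Tick traces straight down from the component and, on a hit, pushes that body along the surface normal with force fading linearly to zero at trace length.
; A hit also sets linear damping, which is never reset here; the angular damping node is disconnected.
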(event EventBeginPlay
  (bind _output_get (Variables|Default|SetParentComponent (Utilities|Array|Get(acopy) (Actor|GetComponentsByClass (Components|GetOwner) "/Script/Engine.PrimitiveComponent"))))
  (Physics|SetSimulatePhysics _output_get true)
  (Development|PrintString "Hello" true true "(R=0.053322,G=1.000000,B=0.071804,A=1.000000)"))

(event EventTick
  (params (DeltaSeconds :type Float%20%28single-precision%29))
  (bind _returnvalue (Transformation|GetWorldLocation))
  (bind (_outhit _returnvalue_2) (Collision|LineTraceByChannel _returnvalue (- _returnvalue (Math|Vector|MakeVector 0.0 0.0 (Variables|Default|GettraceLength))) "TraceTypeQuery1" false 0 "None"))
  (if _returnvalue_2
    (Physics|AddForce (Variables|Default|GetParentComponent) (* (.ImpactNormal (Collision|BreakHitResult _outhit)) (Math|Float|Lerp (Variables|Default|GethoverForce) 0.0 (/ (Math|Vector|VectorLength (- (.Location (Collision|BreakHitResult _outhit)) (Transformation|GetWorldLocation))) (Variables|Default|GettraceLength)))) "None" false)
    (Class|PrimitiveComponent|SetLinearDamping (Variables|Default|GetParentComponent) (Variables|Default|GetlinearDump))))