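; Actor component that makes its owner's first primitive component bob up and down.
; BeginPlay caches that component and its starting height, then Tick advances an angle and sets world Z to that height plus a scaled sine, keeping current X and Y.
; The angle steps per frame without delta time and resets to zero once past 350 degrees, short of a full cycle.
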(event EventBeginPlay
  (bind _output_get (Variables|Default|SetParentComponent (Utilities|Array|Get(acopy) (Actor|GetComponentsByClass (Components|GetOwner) "/Script/Engine.PrimitiveComponent"))))
  (Variables|Default|SetinitialHeight (.z (Transformation|GetWorldLocation _output_get))))

(event EventTick
  (params (DeltaSeconds :type Float%20%28single-precision%29))
  (bind _parentcomponent (Variables|Default|GetParentComponent))
  (bind _returnvalue (Transformation|GetWorldLocation _parentcomponent))
  (if (> (Variables|Default|Getlean) 3.5e+02)
    (Variables|Default|Setlean 0.0)
    (else
      (Variables|Default|Setlean (+ (Variables|Default|Getlean) (Variables|Default|GetleanSpeed)))))
  (Transformation|SetWorldLocation _parentcomponent (Math|Vector|MakeVector (.x _returnvalue) (.y _returnvalue) (+ (Variables|Default|GetinitialHeight) (* (Variables|Default|GetleaMultiplier) (Math|Trig|Sin(Degrees) (Variables|Default|Getlean))))) false false))