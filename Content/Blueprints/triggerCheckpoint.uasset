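; Trigger pickup that passes a particle multiplier to its linked checkpoint when overlapped, then destroys itself.
; On any actor overlap it finds CheckPoint actors whose first tag matches its own and calls SetMultiplier with MultiplierParticle.
; Tick yaws the mesh by RotX each frame.
; Unconnected leftover logic covers player-ID checks, toggling rotation on Show actors, and a pulsing mesh scale.
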(event EventTick
  (params (DeltaSeconds :type Float%20%28single-precision%29))
  (Transformation|AddLocalRotation (Variables|Default|GetMesh) (Math|Rotator|MakeRotator 0.0 0.0 (Variables|Default|GetrotX)) false false))

(event EventBeginPlay)

(event Collision|EventActorBeginOverlap
  (params (OtherActor :type Actor%20Object%20Reference))
  (bind _tags (Variables|Actor|GetTags))
  (bind _item (Utilities|Array|Get(acopy) _tags))
  ;[1 1 1] obraca boxa o danym indexie, jesli gracz stoi w triggerze
  (bind _outactors (Actor|GetAllActorsOfClass "/Game/Blueprints/CheckPoint.CheckPoint_C"))
  (for (_ _array_index) _outactors
    (if (Utilities|Name|Equal(Name) (Utilities|Array|Get(acopy) (Variables|/Script/Engine.Actor|GetTags (Utilities|Array|Get(acopy) _outactors _array_index))) _item)
      (Variables|Default|SetrefIndex 0)
      (Development|PrintString (Utilities|String|ToString(Name) _item))
      (Default|SetMultiplier (Utilities|Array|Get(acopy) _outactors _array_index) (Variables|Default|GetmultiplierParticle))
      (Actor|DestroyActor))))

(event Collision|EventActorEndOverlap
  (params (OtherActor :type Actor%20Object%20Reference))
  ;[1 1 1] obraca boxa o danym indexie, jesli gracz stoi w triggerze
)

(fn ConstructionScript)