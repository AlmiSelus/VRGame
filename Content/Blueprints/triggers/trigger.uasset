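; Trigger actor that makes tag-matched Show actors rotate while something overlaps it.
; Begin overlap sets IsRotating on every Show whose first tag equals the trigger's, saving the last matching index.
; End overlap fetches the Show list again and clears IsRotating only at that index.
; The live path ignores which actor overlaps; ThirdPersonCharacter PlayerId checks remain as disconnected, unused logic.
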(event EventBeginPlay)

(event EventActorBeginOverlap
  (params (OtherActor :type Actor%20Object%20Reference))
  (bind _tags (Variables|Actor|GetTags))
  (bind _item (Utilities|Array|Get(acopy) _tags))
  ;[1 1 1] obraca boxa o danym indexie, jesli gracz stoi w triggerze
  (bind _outactors (Actor|GetAllActorsOfClass "/Game/Blueprints/Show.Show_C"))
  (for (_array_element _array_index) _outactors
    (if (Utilities|Name|Equal(Name) (Utilities|Array|Get(acopy) (Variables|/Script/Engine.Actor|GetTags _array_element)) _item)
      (Variables|Default|SetrefIndex _array_index)
      (Development|PrintString (Utilities|String|ToString(Name) _item))
      (Variables|/Game/Blueprints/Show.Show_C|SetisRotating (Utilities|Array|Get(acopy) _outactors _array_index) true))))

(event Collision|EventActorEndOverlap
  (params (OtherActor :type Actor%20Object%20Reference))
  ;[1 1 1] obraca boxa o danym indexie, jesli gracz stoi w triggerze
  (bind _outactors (Actor|GetAllActorsOfClass "/Game/Blueprints/Show.Show_C"))
  (Variables|/Game/Blueprints/Show.Show_C|SetisRotating (Utilities|Array|Get(acopy) _outactors (Variables|Default|GetrefIndex)) false))

(fn ConstructionScript)