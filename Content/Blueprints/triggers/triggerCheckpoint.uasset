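; Checkpoint trigger pickup that passes its particle multiplier to a referenced checkpoint when any actor overlaps it.
; On overlap it calls SetMultiplier on RefCheckpoint, destroys itself and plays a positive beep.
; Tick yaws the mesh by RotX, and the RepNotify for RefCheckpoint is empty.
; Disconnected leftovers hold player-ID checks toggling rotation of Show actors, a tag-based checkpoint lookup and a pulsing scale animation.
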(event EventTick
  (params (DeltaSeconds :type Float%20%28single-precision%29))
  (Transformation|AddLocalRotation (Variables|Default|GetMesh) (Math|Rotator|MakeRotator 0.0 0.0 (Variables|Default|GetrotX)) false false))

(event EventBeginPlay)

(event Collision|EventActorBeginOverlap
  (params (OtherActor :type Actor%20Object%20Reference))
  (Default|SetMultiplier (Variables|Default|GetrefCheckpoint) (Variables|Default|GetmultiplierParticle))
  (Actor|DestroyActor)
  ;[1 1 1] obraca boxa o danym indexie, jesli gracz stoi w triggerze
  (Audio|PlaySoundatLocation "/Game/Sounds/positive_beep.positive_beep" (Transformation|GetWorldLocation (Variables|Default|GetStaticMesh))))

(event Collision|EventActorEndOverlap
  (params (OtherActor :type Actor%20Object%20Reference))
  ;[1 1 1] obraca boxa o danym indexie, jesli gracz stoi w triggerze
)

(fn ConstructionScript)

(fn OnRepRefCheckpoint)