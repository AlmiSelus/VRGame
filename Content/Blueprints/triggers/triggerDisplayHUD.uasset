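; One-shot trigger actor that hands a HUD widget class to the player character when it walks into the trigger.
; On overlap while active, it identifies the Third Person Character by switching on the class display name string, then clears its active flag.
; It then passes its HudClass to the character's SetGestureWidget, prints a debug message and destroys itself.
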(event EventBeginPlay)

(event Collision|EventActorBeginOverlap
  (params (OtherActor :type Actor%20Object%20Reference))
  (if (Variables|Default|GetisActice)
    (Variables|Default|SetSourceActorObject OtherActor)
    (bind _asactor (Utilities|Casting|CastToActorClass (Utilities|GetClass OtherActor)))
    (switch string (Utilities|GetClassDisplayName _asactor)
      (:ThirdPersonCharacter_c
        (Variables|Default|SetisActice false)
        (bind _asthird_person_character (Utilities|Casting|CastToThirdPersonCharacter (Variables|Default|GetSourceActorObject)))
        (Development|PrintString "HUD")
        (Default|SetGestureWidget _asthird_person_character (Variables|Default|GetHudClass))
        (Actor|DestroyActor)))))

(event EventTick
  (params (DeltaSeconds :type Float%20%28single-precision%29)))

(fn ConstructionScript)