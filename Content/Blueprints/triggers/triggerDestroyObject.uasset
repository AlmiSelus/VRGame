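; Trigger actor that, when the third person character overlaps it, hands that character a destroyable target and then removes itself.
; On overlap it switches on the other actor's class display name, then casts the matching actor to ThirdPersonCharacter.
; It passes its ToDestroy value to the character's SetDestroyable, prints a debug message and destroys the trigger.
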(event EventBeginPlay)

(event Collision|EventActorBeginOverlap
  (params (OtherActor :type Actor%20Object%20Reference))
  (Variables|Default|SetSourceActorObject OtherActor)
  (bind _asactor (Utilities|Casting|CastToActorClass (Utilities|GetClass OtherActor)))
  (switch string (Utilities|GetClassDisplayName _asactor)
    (:ThirdPersonCharacter_c
      (bind _asthird_person_character (Utilities|Casting|CastToThirdPersonCharacter (Variables|Default|GetSourceActorObject)))
      (Default|SetDestroyable _asthird_person_character (Variables|Default|GetToDestroy))
      (Development|PrintString "DESTROY!")
      (Actor|DestroyActor))))

(event EventTick
  (params (DeltaSeconds :type Float%20%28single-precision%29)))

(fn ConstructionScript)