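; LiftableObject is an actor whose static mesh can be lifted toward a target height and made to float.
; It records the mesh's starting world Z at BeginPlay.
; Each Tick, a mesh below roughly the target height eases back toward that start height with a per-frame Lerp.
; Once above that threshold, it adds a FloatIt component if IsFloating is set, then clears the flag.
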(event EventBeginPlay
  (Variables|Default|SetinitialHeight (.z (Transformation|GetWorldLocation (Variables|Default|GetStaticMesh)))))

(event EventActorBeginOverlap
  (params (OtherActor :type Actor%20Object%20Reference)))

(event EventTick
  (params (DeltaSeconds :type Float%20%28single-precision%29))
  (bind _staticmesh (Variables|Default|GetStaticMesh))
  (bind _returnvalue (Transformation|GetWorldLocation _staticmesh))
  (if (> (.z (Transformation|GetWorldLocation (Variables|Default|GetStaticMesh))) (+ (Variables|Default|GettargetHeight) -5.0))
    (if (Variables|Default|GetisFloating)
      (AddComponent|AddFloatIt false)
      (Variables|Default|SetisFloating false))
    (else
      (Transformation|SetWorldLocation (Variables|Default|GetStaticMesh) (Math|Vector|MakeVector (.x _returnvalue) (.y _returnvalue) (Math|Float|Lerp (.z _returnvalue) (Variables|Default|GetinitialHeight) 0.1)) false false))))

(fn ConstructionScript)