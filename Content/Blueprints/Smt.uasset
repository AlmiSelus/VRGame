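; Smt is an actor Blueprint that spins its StaticMesh around the vertical axis.
; Tick calls Play on the RotateMe timeline, whose track value sets the mesh's relative yaw on each update.
; Disconnected leftover logic would trace downward and apply a hover force that fades with distance, along with linear and angular damping, but it never runs.
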(event EventBeginPlay)

(event EventActorBeginOverlap
  (params (OtherActor :type Actor%20Object%20Reference)))

(event EventTick
  (params (DeltaSeconds :type Float%20%28single-precision%29))
  (bind _newtrack_3 (Timeline|RotateMe Play)
    (:Update
      (Transformation|SetRelativeRotation (Variables|Default|GetStaticMesh) (Math|Rotator|MakeRotator 0.0 0.0 _newtrack_3) false false))))

(fn ConstructionScript)