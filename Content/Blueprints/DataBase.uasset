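; DataBase is a shared manager actor for a two-player game that tracks points, assigns player identities and reacts to player proximity.
; setPlayerIDs numbers the two ThirdPersonCharacters and gives each the SplineBP with the matching Id via FindSpline.
; While AllConected is false, Tick re-fetches the players and toggles rotation on the first Show2 actor according to their distance.
; AddPoints accumulates Points, whose OnRep handler is empty.
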(event Custom|AddPoints
  (params (Amount :type Integer))
  ;[1 1 1] DodajPunkty
  (Variables|Default|SetPoints (+ Amount (Variables|Default|GetPoints))))

(event Custom|setPlayerIDs
  (Development|PrintString "Ustawiamy ID" true true "(R=0.000000,G=0.660000,B=1.000000,A=1.000000)" 1e+01)
  (bind _outactors (Actor|GetAllActorsOfClass "/Game/Blueprints/ThirdPersonCharacter.ThirdPersonCharacter_C"))
  (for _index (range 0 1)
    (Development|PrintString (Utilities|String|BuildString(Integer) "" (Utilities|String|BuildString(Integer) "" "index: " _index " got ID:") (+ _index 1)) true true "(R=0.000000,G=0.660000,B=1.000000,A=1.000000)" 4.0)
    (bind _output_get (Variables|/Game/Blueprints/ThirdPersonCharacter.ThirdPersonCharacter_C|SetplayerId (Utilities|Array|Get(acopy) _outactors _index) (+ _index 1)))
    (bind _spline (CallFunction|FindSpline _output_get))
    (Variables|/Game/Blueprints/ThirdPersonCharacter.ThirdPersonCharacter_C|SetSplinePath (Utilities|Array|Get(acopy) _outactors _index) _spline)))

(event EventBeginPlay)

(event EventActorBeginOverlap
  (params (OtherActor :type Actor%20Object%20Reference)))

(event EventTick
  (params (DeltaSeconds :type Float%20%28single-precision%29))
  (if (not (Variables|Default|GetallConected))
    (bind _outactors (Actor|GetAllActorsOfClass "/Game/Blueprints/ThirdPersonCharacter.ThirdPersonCharacter_C"))
    (bind _output_get (Variables|Default|SetrefPlayers _outactors))
    (if (== (Utilities|Array|Length _output_get) 2)
      (if (< (Transformation|GetDistanceTo (Utilities|Array|Get(acopy) (Variables|Default|GetrefPlayers)) (Utilities|Array|Get(acopy) (Variables|Default|GetrefPlayers) 1)) 3e+02)
        (bind _outactors_2 (Actor|GetAllActorsOfClass "/Game/Blueprints/Show2.Show2_C"))
        (Variables|/Game/Blueprints/Show2.Show2_C|SetisRotating (Utilities|Array|Get(acopy) _outactors_2) true)
        (else
          (bind _outactors_3 (Actor|GetAllActorsOfClass "/Game/Blueprints/Show2.Show2_C"))
          (Variables|/Game/Blueprints/Show2.Show2_C|SetisRotating (Utilities|Array|Get(acopy) _outactors_3) false))))))

(fn ConstructionScript)

(fn OnRepPoints)

(fn FindSpline
  (params (id :type Integer))
  (bind _outactors (Actor|GetAllActorsOfClass "/Game/Blueprints/SplineBP.SplineBP_C"))
  (for _array_element _outactors
    (if (== (Variables|/Game/Blueprints/SplineBP.SplineBP_C|Getid _array_element) id)
      (bind _output_get (LocalVariables|SetretSpline _array_element))))
  (return _output_get))