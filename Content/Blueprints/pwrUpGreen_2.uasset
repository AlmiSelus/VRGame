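; Green power-up pickup actor that awards a point when a projectile or the third-person character overlaps it.
; The overlap event identifies the other actor by matching its class display name as a string.
; It calls AddPoints on the first DataBase actor found in the level, prints a Polish message and destroys itself.
; The message announces red and ten points, which differs from the pickup's name and the single point added.
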(event EventBeginPlay)

(event Collision|EventActorBeginOverlap
  (params (OtherActor :type Actor%20Object%20Reference))
  (Variables|Default|SetSourceActorObject OtherActor)
  (bind _asactor (Utilities|Casting|CastToActorClass (Utilities|GetClass OtherActor)))
  (switch string (Utilities|GetClassDisplayName _asactor)
    (:projectile_c
      _)
    (:ThirdPersonCharacter_c
      _))
  (bind _outactors (Actor|GetAllActorsOfClass "/Game/Blueprints/DataBase.DataBase_C"))
  (Default|AddPoints (Utilities|Array|Get(acopy) _outactors) 1)
  (Development|PrintString (Utilities|String|Append "czerwony + " "10" " punktow!"))
  (Actor|DestroyActor))

(fn ConstructionScript)